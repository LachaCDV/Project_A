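; BP_Unit is a grid unit actor whose skeletal mesh and anim class come from default data for its unit type.
; It walks tile paths by replaying a timeline per tile, adding a jump on height changes and firing start, new-tile and finish events.
; Hover and selection tint the mesh through a material parameter.
; A line-of-sight collision mesh matches the grid's tile shape, size and rotation.
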(event Custom|Event_Follow_Path
  (params (Path :type Array%20of%20Int%20Point%20Structures))
  (if (> (Utilities|Array|Length Path) 0)
    (Variables|Default|SetCurrent%20Path%20To%20Follow Path)
    (Default|CallOnUnitStartedWalking self)
    (CallFunction|ContinuetoFolllowPath)))

(event Custom|Continue_To_Folllow_Path
  (bind _grid (Variables|Default|GetGrid))
  (bind _current_path_to_follow (Variables|Default|GetCurrent%20Path%20To%20Follow))
  (bind _timeline_unit_movement (Variables|Default|GetTimeline_Unit_Movement))
  (bind _output (Utilities|Array|Get(acopy) _current_path_to_follow))
  (bind _gridtiles (Variables|/Game/Gierka/Blueprints/Core/Grid/BP_Grid.BP_Grid_C|GetGridTiles _grid))
  (bind _value (Utilities|Map|Find _gridtiles _output))
  (bind _transform (Utilities|Struct|BreakS_TileData _value))
  (if (> (Utilities|Array|Length (Variables|Default|GetCurrent%20Path%20To%20Follow)) 0)
    (CallFunction|SetAnimationState "NewEnumerator1")
    (Variables|Default|SetPrevious%20Transform (Transformation|GetActorTransform))
    (Variables|Default|SetNext%20Transform (Math|Transform|MakeTransform (.location _transform) (Math|Rotator|MakeRotator 0.0 0.0 (.yaw (Math|Rotator|FindLookatRotation (.location (Variables|Default|GetPrevious%20Transform)) (.location _transform)))) "1.000000,1.000000,1.000000"))
    (Components|Timeline|SetPlayRate _timeline_unit_movement (/ (Components|Timeline|GetTimelineLength _timeline_unit_movement) (Variables|Default|GetMoveDurationPerTile)))
    (bind (_direction _location_alpha _rotation_alpha _track_jump) (Timeline|Timeline_Unit_Movement PlayFromStart)
      (:Update
        (Transformation|SetActorLocationAndRotation (+ (Math|Vector|Lerp(Vector) (.location (Variables|Default|GetPrevious%20Transform)) (.location (Variables|Default|GetNext%20Transform)) _location_alpha) (Math|Vector|MakeVector 0.0 0.0 (select (Math|Float|NearlyEqual(Float) (.z (.location (Variables|Default|GetPrevious%20Transform))) (.z (.location (Variables|Default|GetNext%20Transform))) 5.0) 0.0 _track_jump))) (Math|Rotator|Lerp(Rotator) (.rotation (Variables|Default|GetPrevious%20Transform)) (.rotation (Variables|Default|GetNext%20Transform)) _rotation_alpha true)))
      (:Finished
        (Default|CallOnUnitReachNewTile self (Utilities|Array|Get(acopy) (Variables|Default|GetCurrent%20Path%20To%20Follow)))
        (Utilities|Array|RemoveIndex (Variables|Default|GetCurrent%20Path%20To%20Follow))
        (CallFunction|ContinuetoFolllowPath)))
    (else
      (CallFunction|SetAnimationState "NewEnumerator0")
      (Default|CallOnUnitFinishedWalking self))))

(event EventBeginPlay
  (CallFunction|SetAnimationState "NewEnumerator0"))

(fn ConstructionScript
  (bind _unit_data (CallFunction|GetDefaultUnitDatafromUnitType (Variables|Default|GetUnitType)))
  (CallFunction|SetUnitData _unit_data)
  (CallFunction|UpdateVisualwhenHoveredorSelected))

(fn UpdateVisualwhenHoveredorSelected
  (Rendering|Material|SetVectorParameterValueonMaterials (Variables|Default|GetSkeletalMesh) "Color Multiply" (Math|Conversions|ToVector(LinearColor) (* (* (select (Variables|Default|GetIs%20Selected) "(R=0.186899,G=0.970151,B=1.000000,A=1.000000)" "(R=1.000000,G=1.000000,B=1.000000,A=1.000000)") (select (Variables|Default|GetIs%20Hovered) 2.5 1.0)) (select (Variables|Default|GetIs%20Selected) 2.5 1.0)))))

(fn SetIsHovered
  (params (Is%20Hovered :type Boolean))
  (Variables|Default|SetIs%20Hovered Is%20Hovered)
  (CallFunction|UpdateVisualwhenHoveredorSelected))

(fn SetIsSelected
  (params (Is%20Selected :type Boolean))
  (Variables|Default|SetIs%20Selected Is%20Selected)
  (CallFunction|UpdateVisualwhenHoveredorSelected))

(fn SetUnitData
  (params (Data :type S%20Unit%20Data%20Structure%20%28by%20ref%29))
  (bind _skeletalmesh (Variables|Default|GetSkeletalMesh))
  (bind _output_get (Variables|Default|SetUnit%20Data Data))
  (Class|SkinnedMeshComponent|SetSkeletalMesh _skeletalmesh (.Mesh (Utilities|Struct|BreakS_UnitData_Assets (.Assets (Utilities|Struct|BreakS_UnitData _output_get)))) true)
  (Class|SkeletalMeshComponent|SetAnimClass _skeletalmesh (.AnimBlueprint (Utilities|Struct|BreakS_UnitData_Assets (.Assets (Utilities|Struct|BreakS_UnitData _output_get))))))

(fn SetAnimationState
  (params (State :type E_UnitAnimationState%20Enum :default "NewEnumerator0"))
  (Class|BPLUnitAnimation|SetUnitAnimationState(Message) (Components|SkeletalMesh|GetAnimInstance (Variables|Default|GetSkeletalMesh)) State))

(fn SetGrid
  (params (Grid :type BP%20Grid%20Object%20Reference))
  (bind _collision_lineofsight (Variables|Default|GetCollision_LineOfSight))
  (Variables|Default|SetGrid Grid)
  (Components|StaticMesh|SetStaticMesh _collision_lineofsight (.Mesh (Utilities|Struct|BreakS_GridShapeData (Default|GetCurrentShapeData (Variables|Default|GetGrid)))))
  (Transformation|SetAbsolute _collision_lineofsight false true true)
  (Transformation|SetWorldScale3D (Variables|Default|GetCollision_LineOfSight) (Math|Vector|MakeVector (.x (/ (Variables|/Game/Gierka/Blueprints/Core/Grid/BP_Grid.BP_Grid_C|GetGridTileSize (Variables|Default|GetGrid)) (.MeshSize (Utilities|Struct|BreakS_GridShapeData (Default|GetCurrentShapeData (Variables|Default|GetGrid)))))) (.y (/ (Variables|/Game/Gierka/Blueprints/Core/Grid/BP_Grid.BP_Grid_C|GetGridTileSize (Variables|Default|GetGrid)) (.MeshSize (Utilities|Struct|BreakS_GridShapeData (Default|GetCurrentShapeData (Variables|Default|GetGrid)))))) (.z (Transformation|GetWorldScale (Variables|Default|GetCollision_LineOfSight)))))
  (Transformation|SetWorldRotation (Variables|Default|GetCollision_LineOfSight) (Default|GetTileRotationfromGridIndex (Variables|Default|GetGrid) (Variables|Default|GetIndex)) false false))

(fn SetGridIndex
  (params (Index :type Int%20Point%20Structure))
  (Variables|Default|SetIndex Index)
  (Transformation|SetWorldRotation (Variables|Default|GetCollision_LineOfSight) (Default|GetTileRotationfromGridIndex (Variables|Default|GetGrid) (Variables|Default|GetIndex)) false false))