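; Grid visual actor that renders the tile grid through two child instanced-mesh actors, a flat view and a tactical view.
; Tile updates replace instances by index, with the flat view showing only walkable tiles at a ground offset.
; Tactical tiles are thick meshes, Z-scaled down to the lowest recorded tile height and colored by type.
; Tactical mode hides "NotTactical" actors and lazily regenerates its tiles when flagged stale.
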(event EventBeginPlay
  (Actor|Tick|SetActorTickEnabled false))

(event Collision|EventActorBeginOverlap
  (params (OtherActor :type Actor%20Object%20Reference)))

(event EventTick
  (params (DeltaSeconds :type Float%20%28single-precision%29)))

(fn ConstructionScript)

(fn InitializeGridVisual
  (params (Grid :type BP%20Grid%20Object%20Reference))
  (Variables|Default|SetGrid Grid)
  (Variables|Default|SetGrid%20Mesh%20Inst (.AsBP%20Grid%20Mesh%20Inst (Utilities|Casting|CastToBP_GridMeshInst (Variables|/Script/Engine.ChildActorComponent|GetChildActor (Variables|Default|GetChildActor_GridMeshInst)))))
  (Variables|Default|SetGrid%20Mesh%20Inst%20Tactical (.AsBP%20Grid%20Mesh%20Inst (Utilities|Casting|CastToBP_GridMeshInst (Variables|/Script/Engine.ChildActorComponent|GetChildActor (Variables|Default|GetChildActor_GridMeshInst_Tactical)))))
  ;[1 1 1] setup the components
  (Default|InitialazeGridMeshInst (Variables|Default|GetGrid%20Mesh%20Inst) (.FlatMesh (Utilities|Struct|BreakS_GridShapeData (Default|GetCurrentShapeData (Variables|Default|GetGrid)))) (.FlatMaterial (Utilities|Struct|BreakS_GridShapeData (Default|GetCurrentShapeData (Variables|Default|GetGrid)))) false "QueryOnly")
  (Default|InitialazeGridMeshInst (Variables|Default|GetGrid%20Mesh%20Inst%20Tactical) (.Mesh (Utilities|Struct|BreakS_GridShapeData (Default|GetCurrentShapeData (Variables|Default|GetGrid)))) (.MeshMaterial (Utilities|Struct|BreakS_GridShapeData (Default|GetCurrentShapeData (Variables|Default|GetGrid)))) true "QueryOnly")
  ;[1 1 1] center grid in world
  (Transformation|SetActorLocation "0, 0, 0" false false)
  (CallFunction|SetOffsetfromGround (Variables|Default|GetOffset%20From%20Ground))
  (CallFunction|SetGridLowestZ 999999.0)
  (CallFunction|SetIsTactical (Variables|Default|GetIs%20Tactical)))

(fn SetOffsetfromGround
  (params (Offset :type Float%20%28double-precision%29))
  (Variables|Default|SetOffset%20From%20Ground Offset)
  (Transformation|SetRelativeLocation (Variables|Default|GetChildActor_GridMeshInst) (Math|Vector|MakeVector 0.0 0.0 (Variables|Default|GetOffset%20From%20Ground)) false false))

(fn DestroyGridVisual
  (bind _grid_mesh_inst_tactical (Variables|Default|GetGrid%20Mesh%20Inst%20Tactical))
  (bind _grid_mesh_inst (Variables|Default|GetGrid%20Mesh%20Inst))
  (Utilities|FlowControl|Sequence
    (:then_0
      (Utilities|IsValid _grid_mesh_inst
        (:Is%20Valid
          (Default|ClearInstances _grid_mesh_inst))))
    (:then_1
      (Utilities|IsValid _grid_mesh_inst_tactical
        (:Is%20Valid
          (Default|ClearInstances _grid_mesh_inst_tactical))))
    (:then_2
      (CallFunction|SetGridLowestZ 999999.0))))

(fn UpdateTileVisual
  (params (Data :type S%20Tile%20Data%20Structure))
  (Utilities|FlowControl|Sequence
    (:then_0
      (Default|RemoveInstance (Variables|Default|GetGrid%20Mesh%20Inst) (.index Data))
      (if (CallFunction|IsTileWalkable (.type Data))
        (Default|AddInstance (Variables|Default|GetGrid%20Mesh%20Inst) (.index Data) (.transform Data) (.states Data) (.type Data))))
    (:then_1
      (CallFunction|UpdateTileVisualTactical Data))))

(fn UpdateTileVisualTactical
  (params (Data :type S%20Tile%20Data%20Structure))
  (bind _grid (Variables|Default|GetGrid))
  (bind (_location _rotation _scale) (Math|Transform|BreakTransform (.transform Data)))
  (bind _location_2 (Math|Transform|BreakTransform (.transform Data)))
  (bind _returnvalue (Default|GetCurrentShapeData _grid))
  (bind _meshsize (Utilities|Struct|BreakS_GridShapeData _returnvalue))
  (bind _z (Math|Vector|BreakVector _meshsize))
  (Utilities|FlowControl|Sequence
    (:then_0
      (if (< (.z _location_2) (Variables|Default|GetGrid%20Lowest%20Z))
        (CallFunction|SetGridLowestZ (.z _location_2))))
    (:then_1
      (if (Variables|Default|GetIs%20Tactical)
        (Default|RemoveInstance (Variables|Default|GetGrid%20Mesh%20Inst%20Tactical) (.index Data))
        (if (Utilities|Enum|NotEqual(Enum) (.type Data) "NewEnumerator0")
          (Default|AddInstance (Variables|Default|GetGrid%20Mesh%20Inst%20Tactical) (.index Data) (Math|Transform|MakeTransform _location _rotation (Math|Vector|MakeVector (.x _scale) (.y _scale) (/ (+ (- (.Z (Math|Vector|BreakVector (.Location (Math|Transform|BreakTransform (.transform Data))))) (Variables|Default|GetGrid%20Lowest%20Z)) _z) _z))) (.states Data) (.type Data)))
        (else
          (Variables|Default|SetNeed%20To%20Re%20Generate%20Tactical%20on%20Next%20Enable true))))))

(fn SetGridLowestZ
  (params (Z :type Float%20%28double-precision%29))
  (Variables|Default|SetGrid%20Lowest%20Z Z)
  (Variables|Default|SetNeed%20To%20Re%20Generate%20Tactical%20on%20Next%20Enable true))

(fn SetIsTactical
  (params (Tactical? :type Boolean))
  (Variables|Default|SetIs%20Tactical Tactical?)
  (Development|SetHiddeninGame (Variables|Default|GetChildActor_GridMeshInst_Tactical) (not (Variables|Default|GetIs%20Tactical)) false)
  (bind _outactors (Actor|GetAllActorswithTag "NotTactical"))
  (for _array_element _outactors
    (Rendering|SetActorHiddenInGame _array_element (Variables|Default|GetIs%20Tactical)))
  (if (and (Variables|Default|GetIs%20Tactical) (Variables|Default|GetNeed%20To%20Re%20Generate%20Tactical%20on%20Next%20Enable))
    (Variables|Default|SetNeed%20To%20Re%20Generate%20Tactical%20on%20Next%20Enable false)
    (bind _values (Utilities|Map|Values (Variables|/Game/Gierka/Blueprints/Core/Grid/BP_Grid.BP_Grid_C|GetGridTiles (Variables|Default|GetGrid))))
    (for _array_element_2 _values
      (CallFunction|UpdateTileVisualTactical _array_element_2))))