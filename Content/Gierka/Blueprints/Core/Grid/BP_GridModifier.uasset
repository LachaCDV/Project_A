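; BP_GridModifier is a level-placed marker that tags grid space with a tile type, such as obstacle, extra movement cost or flying-units-only.
; Its construction script takes the mesh and flat material from the Shape's data, then colors it by Type as a filled tile.
; It sets one custom trace channel to overlap and another to block, and hides the actor in game.
; The event graph holds no logic.
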(event EventBeginPlay)

(event Collision|EventActorBeginOverlap
  (params (OtherActor :type Actor%20Object%20Reference)))

(event EventTick
  (params (DeltaSeconds :type Float%20%28single-precision%29)))

(fn ConstructionScript
  (bind _shape (Variables|Default|GetShape))
  (bind _staticmesh (Variables|Default|GetStaticMesh))
  (bind _data (CallFunction|GetShapeData _shape))
  (Components|StaticMesh|SetStaticMesh _staticmesh (.mesh _data))
  (Rendering|Material|SetMaterial _staticmesh 0 (.flatmaterial _data))
  (Rendering|Material|SetVectorParameterValueonMaterials _staticmesh "Color" (Utilities|Select :Index (Variables|Default|GetType) :NewEnumerator0 "0, 0, 0" :NewEnumerator1 (Math|Conversions|ToVector(LinearColor) "(R=1.000000,G=1.000000,B=1.000000,A=1.000000)") :NewEnumerator2 (Math|Conversions|ToVector(LinearColor) "(R=1.000000,G=0.000000,B=0.111830,A=1.000000)") :NewEnumerator3 (Math|Conversions|ToVector(LinearColor) "(R=0.000000,G=1.000000,B=0.276372,A=1.000000)") :NewEnumerator4 (Math|Conversions|ToVector(LinearColor) "(R=1.000000,G=0.429789,B=0.000000,A=1.000000)") :NewEnumerator5 (Math|Conversions|ToVector(LinearColor) "(R=1.000000,G=0.791493,B=0.000000,A=1.000000)")))
  (Rendering|Material|SetScalarParameterValueonMaterials _staticmesh "Is Filled" 1.0)
  (Collision|SetCollisionResponsetoChannel _staticmesh "ECC_GameTraceChannel1" "ECR_Overlap")
  (Collision|SetCollisionResponsetoChannel _staticmesh "ECC_GameTraceChannel4" "ECR_Block")
  (Rendering|SetActorHiddenInGame true))