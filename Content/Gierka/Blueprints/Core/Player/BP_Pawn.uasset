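; BP_Pawn is the player's camera pawn, which pans, rotates and zooms on a spring arm.
; Axis inputs move a desired location along the actor's forward and right vectors and adjust a clamped desired zoom, while button presses step the desired yaw left or right.
; Tick smooths location, rotation and arm length toward these targets with interpolation, starting from the values captured at BeginPlay.
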(event EventTick
  (params (DeltaSeconds :type Float%20%28single-precision%29))
  (bind _springarm (Variables|Default|GetSpringArm))
  (Variables|/Script/Engine.SpringArmComponent|SetTargetArmLength _springarm (Math|Interpolation|FInterpTo (Variables|/Script/Engine.SpringArmComponent|GetTargetArmLength _springarm) (Variables|Default|GetZoom_Desire) DeltaSeconds (Variables|Default|GetZoom_Interp)))
  (Transformation|SetActorLocation (Math|Interpolation|VInterpTo (Transformation|GetActorLocation) (Variables|Default|GetLocation_desire) DeltaSeconds (Variables|Default|GetLocation_Interp)) false false)
  (Transformation|SetActorRotation (Math|Interpolation|RInterpTo (Transformation|GetActorRotation) (Variables|Default|GetRotation_desire) DeltaSeconds (Variables|Default|GetRotation_Interp))))

(event EventBeginPlay
  (Variables|Default|SetLocation_desire (Transformation|GetActorLocation))
  (Variables|Default|SetZoom_Desire (Variables|/Script/Engine.SpringArmComponent|GetTargetArmLength (Variables|Default|GetSpringArm)))
  (Variables|Default|SetRotation_desire (Transformation|GetActorRotation)))

(event Input|ActionEvents|InputActionInputAction_Rotation_Right
  (params (Key :type Key%20Structure :default "None"))
  (:Pressed
    (Variables|Default|SetRotation_desire (Math|Rotator|CombineRotators (Variables|Default|GetRotation_desire) (Math|Rotator|MakeRotator 0.0 0.0 (Variables|Default|GetRotation_Speed))))))

(event Input|ActionEvents|InputActionInputAction_Rotation_Left
  (params (Key :type Key%20Structure :default "None"))
  (:Pressed
    (Variables|Default|SetRotation_desire (Math|Rotator|CombineRotators (Variables|Default|GetRotation_desire) (Math|Rotator|MakeRotator 0.0 0.0 (- 0.0 (Variables|Default|GetRotation_Speed)))))))

(event Input|AxisEvents|InputAxisInputAxis_Zoom
  (params (AxisValue :type Float%20%28single-precision%29))
  (Variables|Default|SetZoom_Desire (Math|Float|Clamp(Float) (+ (Variables|Default|GetZoom_Desire) (* AxisValue (Variables|Default|GetZoom_Speed))) (Variables|Default|GetZoom_Min) (Variables|Default|GetZoom_Max))))

(event Input|AxisEvents|InputAxisInputAxis_Forward
  (params (AxisValue :type Float%20%28single-precision%29))
  (Variables|Default|SetLocation_desire (+ (Variables|Default|GetLocation_desire) (* (* AxisValue (Variables|Default|GetLocation_Speed)) (Transformation|GetActorForwardVector)))))

(event Input|AxisEvents|InputAxisInputAxis_Right
  (params (AxisValue :type Float%20%28single-precision%29))
  (Variables|Default|SetLocation_desire (+ (Variables|Default|GetLocation_desire) (* (* AxisValue (Variables|Default|GetLocation_Speed)) (Transformation|GetActorRightVector)))))

(fn ConstructionScript)