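; BP_PlayerActions turns mouse input into actions on the tactical grid and tracks the hovered and selected tile and unit.
; Each Tick resolves hover by unit trace or grid tile, updating tile states and unit highlights.
; SetSelectedActions spawns swappable action actors for left and right click, which execute on press and on each new tile while held.
; Grid and combat system events refresh the selection when tiles or units change.
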(event Custom|OnHoveredTileChanged
  (bind _selectedaction_rightclick (Variables|Default|GetSelectedAction_RightClick))
  (bind _selectedaction_leftclick (Variables|Default|GetSelectedAction_LeftClick))
  (Utilities|FlowControl|Sequence
    (:then_0
      (Utilities|IsValid _selectedaction_leftclick
        (:Is%20Valid
          (Default|ExecuteHoveredAction _selectedaction_leftclick (Variables|Default|GetHovered%20Tile))
          (if (Variables|Default|GetIsLeftClickDown)
            (Default|ExecuteAction (Variables|Default|GetSelectedAction_LeftClick) (Variables|Default|GetHovered%20Tile))))))
    (:then_1
      (Utilities|IsValid _selectedaction_rightclick
        (:Is%20Valid
          (Default|ExecuteHoveredAction _selectedaction_rightclick (Variables|Default|GetHovered%20Tile))
          (if (Variables|Default|GetIsRightClickDown)
            (Default|ExecuteAction (Variables|Default|GetSelectedAction_RightClick) (Variables|Default|GetHovered%20Tile))))))))

(event EventBeginPlay
  (bind _returnvalue (Actor|GetActorOfClass "/Game/Gierka/Blueprints/Core/Grid/BP_Grid.BP_Grid_C"))
  (Variables|Default|SetGrid _returnvalue)
  (EventDispatchers|BindEventtoOnGridGenerated (Variables|Default|GetGrid) (EventDispatchers|CreateEvent :!event OnGridGenerated))
  (EventDispatchers|BindEventtoOnTileDataUpdated (Variables|Default|GetGrid) (EventDispatchers|CreateEvent :!event OnTileDataUpdated))
  (bind _returnvalue_2 (Actor|GetActorOfClass "/Game/Gierka/Blueprints/Core/Combat/BP_CombatSystem.BP_CombatSystem_C"))
  (bind _output_get (Variables|Default|SetCombat%20System _returnvalue_2))
  (EventDispatchers|BindEventtoOnUnitGridIndexChanged _output_get (EventDispatchers|CreateEvent :!event OnUnitGridIndexChanged))
  (Input|EnableInput (Game|GetPlayerController 0)))

(event EventTick
  (params (DeltaSeconds :type Float%20%28single-precision%29))
  (CallFunction|UpdateHoveredTileandUnit))

(event Input|MouseEvents|LeftMouseButton
  (params (Key :type Key%20Structure :default "None"))
  (bind _selectedaction_leftclick (Variables|Default|GetSelectedAction_LeftClick))
  (:Pressed
    (CallFunction|UpdateHoveredTileandUnit)
    (Variables|Default|SetIsLeftClickDown true)
    (Utilities|IsValid _selectedaction_leftclick
      (:Is%20Valid
        (Default|ExecuteAction _selectedaction_leftclick (Variables|Default|GetHovered%20Tile)))))
  (:Released
    (Variables|Default|SetIsLeftClickDown false)))

(event Input|MouseEvents|RightMouseButton
  (params (Key :type Key%20Structure :default "None"))
  (bind _selectedaction_rightclick (Variables|Default|GetSelectedAction_RightClick))
  (:Pressed
    (CallFunction|UpdateHoveredTileandUnit)
    (Variables|Default|SetIsRightClickDown true)
    (Utilities|IsValid _selectedaction_rightclick
      (:Is%20Valid
        (Default|ExecuteAction _selectedaction_rightclick (Variables|Default|GetHovered%20Tile)))))
  (:Released
    (Variables|Default|SetIsRightClickDown false)))

(fn ConstructionScript)

(fn UpdateHoveredTileandUnit
  (Utilities|FlowControl|Sequence
    (:then_0
      (bind _unit (CallFunction|GetUnitUnderCursor))
      (if (!= _unit (Variables|Default|GetHovered%20Unit))
        (Utilities|FlowControl|Sequence
          (:then_0
            (Utilities|IsValid (Variables|Default|GetHovered%20Unit)
              (:Is%20Valid
                (Default|SetIsHovered (Variables|Default|GetHovered%20Unit) false))))
          (:then_1
            (bind _output_get (Variables|Default|SetHovered%20Unit _unit))
            (Utilities|IsValid _output_get
              (:Is%20Valid
                (Default|SetIsHovered _output_get true)))))))
    (:then_1
      (Utilities|IsValid (Variables|Default|GetHovered%20Unit)
        (:Is%20Valid
          (LocalVariables|SetNew%20Index (Variables|/Game/Gierka/Blueprints/Core/Units/BP_Unit.BP_Unit_C|GetIndex (Variables|Default|GetHovered%20Unit))))
        (:Is%20Not%20Valid
          (bind _index (Default|GetTileIndexUnderCursor (Variables|Default|GetGrid)))
          (LocalVariables|SetNew%20Index _index)))
      (if (!= (LocalVariables|GetNew%20Index) (Variables|Default|GetHovered%20Tile))
        (Default|RemoveStatefromTile (Variables|Default|GetGrid) (Variables|Default|GetHovered%20Tile) "NewEnumerator1")
        (Variables|Default|SetHovered%20Tile (LocalVariables|GetNew%20Index))
        (Default|AddStatetoTile (Variables|Default|GetGrid) (Variables|Default|GetHovered%20Tile) "NewEnumerator1")
        (CallFunction|OnHoveredTileChanged)))))

(fn SetSelectedActions
  (params (LeftAction :type BP%20Action%20Class%20Reference) (RightAction :type BP%20Action%20Class%20Reference))
  (Utilities|FlowControl|Sequence
    (:then_0
      (Utilities|IsValid (Variables|Default|GetSelectedAction_LeftClick)
        (:Is%20Valid
          (Actor|DestroyActor (Variables|Default|GetSelectedAction_LeftClick))
          (Variables|Default|SetSelectedAction_LeftClick 0))
        (:Is%20Not%20Valid
          _))
      (if (Utilities|IsValidClass LeftAction)
        (bind _returnvalue (Game|SpawnActorfromClass LeftAction (Math|Transform|MakeTransform "0, 0, 0" "0, 0, 0" "1.000000,1.000000,1.000000") "AlwaysSpawn" 0 self 0))
        (Variables|Default|SetSelectedAction_LeftClick _returnvalue)))
    (:then_1
      (Utilities|IsValid (Variables|Default|GetSelectedAction_RightClick)
        (:Is%20Valid
          (Actor|DestroyActor (Variables|Default|GetSelectedAction_RightClick))
          (Variables|Default|SetSelectedAction_RightClick 0))
        (:Is%20Not%20Valid
          _))
      (if (Utilities|IsValidClass RightAction)
        (bind _returnvalue_2 (Game|SpawnActorfromClass RightAction (Math|Transform|MakeTransform "0, 0, 0" "0, 0, 0" "1.000000,1.000000,1.000000") "AlwaysSpawn" 0 self 0))
        (Variables|Default|SetSelectedAction_RightClick _returnvalue_2)))
    (:then_2
      (Default|CallOnSelectedActionsChanged (Variables|Default|GetSelectedAction_LeftClick) (Variables|Default|GetSelectedAction_RightClick)))))

(fn GetUnitUnderCursor
  (params (PlayerIndex :type Integer))
  (bind _returnvalue (Game|GetPlayerController PlayerIndex))
  (bind (_hitresult _returnvalue_2) (Game|Player|GetHitResultUnderCursorbyChannel _returnvalue "TraceTypeQuery5" false))
  (if _returnvalue_2 ; Mouse over unit?
    (return (.AsBP%20Unit (Utilities|Casting|CastToBP_Unit (.HitActor (Collision|BreakHitResult _hitresult)))))
    (else
      (bind _index (Default|GetTileIndexUnderCursor (Variables|Default|GetGrid) PlayerIndex)) ; Not hovering unit itself but tile with unit on it
      (return (.UnitOnTile (Utilities|Struct|BreakS_TileData (.Value (Utilities|Map|Find (Variables|/Game/Gierka/Blueprints/Core/Grid/BP_Grid.BP_Grid_C|GetGridTiles (Variables|Default|GetGrid)) _index))))))))

(fn SetSelectedTileandUnit
  (params (Index :type Int%20Point%20Structure) (Force :type Boolean))
  (Utilities|FlowControl|Sequence
    (:then_0
      (if (or (!= (Variables|Default|GetSelected%20Tile) Index) Force)
        (Default|RemoveStatefromTile (Variables|Default|GetGrid) (Variables|Default|GetSelected%20Tile) "NewEnumerator2")
        (Variables|Default|SetSelected%20Tile Index)
        (Default|AddStatetoTile (Variables|Default|GetGrid) (Variables|Default|GetSelected%20Tile) "NewEnumerator2")
        (else
          (Default|RemoveStatefromTile (Variables|Default|GetGrid) (Variables|Default|GetSelected%20Tile) "NewEnumerator2")
          (Variables|Default|SetSelected%20Tile (Utilities|Struct|MakeIntPoint -999 -999))))
      (Default|CallOnSelectedTileChanged (Variables|Default|GetSelected%20Tile)))
    (:then_1
      (LocalVariables|SetNew%20Unit (.UnitOnTile (Utilities|Struct|BreakS_TileData (.Value (Utilities|Map|Find (Variables|/Game/Gierka/Blueprints/Core/Grid/BP_Grid.BP_Grid_C|GetGridTiles (Variables|Default|GetGrid)) (Variables|Default|GetSelected%20Tile))))))
      (if (or (!= (Variables|Default|GetSelected%20Unit) (LocalVariables|GetNew%20Unit)) Force)
        (Utilities|FlowControl|Sequence
          (:then_0
            (Utilities|IsValid (Variables|Default|GetSelected%20Unit)
              (:Is%20Valid
                (Default|SetIsSelected (Variables|Default|GetSelected%20Unit) false))))
          (:then_1
            (bind _output_get (Variables|Default|SetSelected%20Unit (LocalVariables|GetNew%20Unit)))
            (Utilities|IsValid _output_get
              (:Is%20Valid
                (Default|SetIsSelected _output_get true)))))))))

(fn OnGridGenerated
  (if (Default|IsIndexValid (Variables|Default|GetGrid) (Variables|Default|GetSelected%20Tile))
    (CallFunction|SetSelectedTileandUnit (Variables|Default|GetSelected%20Tile) true)
    (else
      (CallFunction|SetSelectedTileandUnit (Utilities|Struct|MakeIntPoint -999 -999) false))))

(fn OnTileDataUpdated
  (params (Index :type Int%20Point%20Structure))
  (if (Class|KismetMathLibrary|EqualIntPointIntPoint Index (Variables|Default|GetSelected%20Tile))
    (CallFunction|OnGridGenerated)))

(fn OnUnitGridIndexChanged
  (params (Unit :type BP%20Unit%20Object%20Reference))
  (if (== Unit (Variables|Default|GetSelected%20Unit))
    (CallFunction|SetSelectedTileandUnit (Variables|/Game/Gierka/Blueprints/Core/Units/BP_Unit.BP_Unit_C|GetIndex Unit) false)))